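; Dynamic sky actor that sets lighting, atmosphere, fog, clouds and precipitation from time of day and weather condition.
; The construction script creates the sky sphere's dynamic material, then runs ConfigureDynamicSky.
; TimeOfDay rotates sun and moon and switches day/night settings, while weather selects a data asset, cloud parameters and Niagara rain or snow.
; Rain, thunderstorm and snow force TimeOfDay to late morning, overriding the set time.
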(event EventBeginPlay)

(event Collision|EventActorBeginOverlap
  (params (OtherActor :type Actor%20Object%20Reference)))

(event EventTick
  (params (DeltaSeconds :type Float%20%28single-precision%29)))

(event EventConfigureDynamicSky
  (Utilities|FlowControl|Sequence
    (:then_0
      (Weather|HandleWeatherSettings))
    (:then_1
      (Settings|HandleSunRotation)
      (Nigth|HandleNight))
    (:then_2
      (Settings|HandleVisibility))
    (:then_3
      (Clouds|HandleClouds))))

(fn ConstructionScript
  (Settings|InitSkySphere)
  (Class|WSkySystemBase|ConfigureDynamicSky))

(fn HandleSunRotation
  (Transformation|SetWorldRotation (Variables|Default|GetSunDirectionalLight) (Math|Rotator|MakeRotator 0.0 (Math|Float|MapRangeUnclamped (Variables|Default|GetTimeOfDay) (Variables|Default|GetSunrise) (Variables|Default|GetSunset) 0.0 -1.8e+02) 0.0) false false))

(fn HandleMoonRotationBeforeSunset
  (Transformation|SetWorldRotation (Variables|Default|GetMonDirectionalLight) (Math|Rotator|MakeRotator 0.0 (Math|Float|MapRangeUnclamped (Variables|Default|GetTimeOfDay) (+ (Variables|Default|GetSunset) 0.3) 24.0 -1.8e+02 -9e+01) 0.0) false false))

(fn HandleMoonRotationBeforeSunrise
  (Transformation|SetWorldRotation (Variables|Default|GetMonDirectionalLight) (Math|Rotator|MakeRotator 0.0 (Math|Float|MapRangeUnclamped (Variables|Default|GetTimeOfDay) 0.0 (- (Variables|Default|GetSunrise) -0.3) -9e+01 0.0) 0.0) false false))

(fn HandleVisibility
  (Rendering|SetVisibility (Variables|Default|GetSunDirectionalLight) (Utilities|IsDayTime) false)
  (Rendering|SetVisibility (Variables|Default|GetMonDirectionalLight) (Utilities|IsNightTime) false)
  (Rendering|Material|SetScalarParameterValue (Variables|Settings|GetMI_DynamicSkySphere) "IsMoonVisible" (Math|Conversions|ToFloat(Boolean) (Utilities|IsNightTime)) :!class /Script/Engine.MaterialInstanceDynamic))

(fn HandleNight
  (Nigth|HandleMoonRotationBeforeSunrise)
  (Nigth|HandleMoonRotationBeforeSunset)
  (Nigth|HandleNightSettings))

(fn HandleNightSettings
  (bind _mondirectionallight (Variables|Default|GetMonDirectionalLight))
  (bind _skyatmosphere (Variables|Default|GetSkyAtmosphere))
  (if (Utilities|IsNightTime)
    (Utilities|FlowControl|Sequence
      (:then_0
        (Rendering|Components|Light|SetIntensity _mondirectionallight (Variables|NightSettings|GetMoonLightIntensity))
        (Rendering|Components|Light|SetLightColor _mondirectionallight (Variables|NightSettings|GetMoonLightColor) true)
        (Class|DirectionalLightComponent|SetLightSourceAngle _mondirectionallight (Variables|NightSettings|GetMoonSourceAngle))
        (Class|LightComponent|SetTemperature _mondirectionallight (Variables|NightSettings|GetMoonTemperature)))
      (:then_1
        (Class|SkyAtmosphereComponent|SetRayleighScattering _skyatmosphere (Variables|NightSettings|GetNigthSkyRayleighScattering))
        (Class|SkyAtmosphereComponent|SetMultiScatteringFactor _skyatmosphere (Variables|NightSettings|GetNightSkyMultiScattering))))
    (else
      (Weather|HandleWeatherSettings))))

(fn InitSkySphere
  (bind _returnvalue (Rendering|Material|CreateDynamicMaterialInstance (Variables|Default|GetSM_SkySphere) 0 0 "None" :!class /Script/Engine.PrimitiveComponent))
  (Variables|Settings|SetMI_DynamicSkySphere _returnvalue))

(fn ToggleClouds
  (params (Show :type Boolean))
  (Rendering|Material|SetScalarParameterValue (Variables|Settings|GetMI_DynamicSkySphere) "IsCloudVisible" (Math|Conversions|ToFloat(Boolean) Show) :!class /Script/Engine.MaterialInstanceDynamic))

(fn HandleClouds
  (switch Utilities|FlowControl|Switch|SwitchonEWeatherConditions (Variables|Default|GetWeatherCondition)
    (:Clear
      (Clouds|ToggleClouds false))
    (:Rain
      (Clouds|SetCloudRainySettings :!label _label)
      (Clouds|ToggleClouds true :!label _label_2))
    (:Clouds
      (Clouds|SetCloudSunnySettings :!label _label_3)
      (goto _label_2))
    (:Thunderstorm
      (goto _label))
    (:Drizzle
      (goto _label_3))
    (:Snow
      (goto _label_3))))

(fn SetCloudSunnySettings
  (Rendering|Material|SetVectorParameterValue (Variables|Settings|GetMI_DynamicSkySphere) "CloudSettings" (Utilities|Struct|MakeLinearColor 1.0 (Variables|Clouds|GetCloudPanningSpeed) (Variables|Clouds|GetCloudBrightness) (Math|Float|SelectFloat (Variables|Clouds|GetCloudsDayTimeSkyTineStregth) (Variables|Clouds|GetCloudsNightTimeSkyTineStregth) (Utilities|IsDayTime))) :!class /Script/Engine.MaterialInstanceDynamic))

(fn SetSkyLightSettings
  (if (Utilities|IsDayTime)
    (Rendering|Components|Light|SetIntensity (Variables|Default|GetSkyLight) (Utilities|Struct|BreakS_SkyLightSettings (Variables|/Game/_WeatherVR/DataAssets/BP_Weather_DataAssetBase.BP_Weather_DataAssetBase_C|GetSkyLightSettings (Variables|Weather|GetCurrentWeatherStruct))))))

(fn SetDirectionalLightSettings
  (bind _currentweatherstruct (Variables|Weather|GetCurrentWeatherStruct))
  (bind _sundirectionallight (Variables|Default|GetSunDirectionalLight))
  (bind _directionallightsettings (Variables|/Game/_WeatherVR/DataAssets/BP_Weather_DataAssetBase.BP_Weather_DataAssetBase_C|GetDirectionalLightSettings _currentweatherstruct))
  (bind (_intensity _color _sourceangle _temperature) (Utilities|Struct|BreakS_DirectionalLightSettings _directionallightsettings))
  (if (Utilities|IsDayTime)
    (Rendering|Components|Light|SetIntensity _sundirectionallight _intensity)
    (Rendering|Components|Light|SetLightColor _sundirectionallight _color true)
    (Class|DirectionalLightComponent|SetLightSourceAngle _sundirectionallight _sourceangle)
    (Class|LightComponent|SetTemperature _sundirectionallight _temperature)))

(fn HandleWeatherSettings
  (switch Utilities|FlowControl|Switch|SwitchonEWeatherConditions (Variables|Default|GetWeatherCondition)
    (:Clear
      (Variables|Weather|SetCurrentWeatherStruct "/Game/_WeatherVR/DataAssets/DA_Clear.DA_Clear" :!label _label))
    (:Rain
      (Variables|Weather|SetCurrentWeatherStruct "/Game/_WeatherVR/DataAssets/DA_Rainy.DA_Rainy" :!label _label_2)
      (Variables|Default|SetTimeOfDay 11.0 :!label _label_3))
    (:Clouds
      (goto _label))
    (:Thunderstorm
      (goto _label_2))
    (:Drizzle
      (goto _label))
    (:Snow
      (Variables|Weather|SetCurrentWeatherStruct "/Game/_WeatherVR/DataAssets/DA_Snowy.DA_Snowy")
      (goto _label_3)))
  (Utilities|FlowControl|Sequence
    (:then_0
      (Weather|SetSkyLightSettings))
    (:then_1
      (Weather|SetSkyAtmosphereSettings))
    (:then_2
      (Weather|SetDirectionalLightSettings))
    (:then_3
      (Weather|SetExponentialHeightFog))
    (:then_4
      (Weather|ToggleSnow (Utilities|IsSnowing)))
    (:then_5
      (Weather|HandleRain))))

(fn SetSkyAtmosphereSettings
  (bind _currentweatherstruct (Variables|Weather|GetCurrentWeatherStruct))
  (bind _skyatmosphere (Variables|Default|GetSkyAtmosphere))
  (bind _skyatmospheresettings (Variables|/Game/_WeatherVR/DataAssets/BP_Weather_DataAssetBase.BP_Weather_DataAssetBase_C|GetSkyAtmosphereSettings _currentweatherstruct))
  (bind (_multiscattering _rayleighscattering _miescatteringscale _mieabsortionscale _mieanisotropy _arealperspectiveviewdistancescale) (Utilities|Struct|BreakS_SkyAtmosphereSettings _skyatmospheresettings))
  (if (Utilities|IsDayTime)
    (Class|SkyAtmosphereComponent|SetMultiScatteringFactor _skyatmosphere _multiscattering)
    (Class|SkyAtmosphereComponent|SetRayleighScattering _skyatmosphere _rayleighscattering)
    (Class|SkyAtmosphereComponent|SetMieScatteringScale _skyatmosphere _miescatteringscale)
    (Class|SkyAtmosphereComponent|SetMieAbsorptionScale _skyatmosphere _mieabsortionscale)
    (Class|SkyAtmosphereComponent|SetMieAnisotropy _skyatmosphere _mieanisotropy)
    (Class|SkyAtmosphereComponent|SetAerialPespectiveViewDistanceScale _skyatmosphere _arealperspectiveviewdistancescale)))

(fn SetExponentialHeightFog
  (bind _exponentialheightfog (Variables|Default|GetExponentialHeightFog))
  (bind _currentweatherstruct (Variables|Weather|GetCurrentWeatherStruct))
  (bind _exponentialheightfogsettings (Variables|/Game/_WeatherVR/DataAssets/BP_Weather_DataAssetBase.BP_Weather_DataAssetBase_C|GetExponentialHeightFogSettings _currentweatherstruct))
  (bind (_emissivecolor _extinctionscale) (Utilities|Struct|BreakS_ExponentialHeightFogSettings _exponentialheightfogsettings))
  (if (Utilities|IsDayTime)
    (Class|ExponentialHeightFogComponent|SetVolumetricFogEmissive _exponentialheightfog _emissivecolor)
    (Class|ExponentialHeightFogComponent|SetVolumetricFogExtinctionScale _exponentialheightfog _extinctionscale)))

(fn ToggleSnow
  (params (Enable :type Boolean))
  (bind _ns_snow (Variables|Default|GetNS_Snow))
  (Components|Activation|SetAutoActivate _ns_snow Enable)
  (Components|Activation|SetActive _ns_snow Enable Enable))

(fn SetCloudRainySettings
  (bind _rainweathersettings (Variables|Weather|GetRainWeatherSettings))
  (bind (_panningspeed _brightness _skytintstregth) (Utilities|Struct|BreakS_RainSettings _rainweathersettings))
  (Rendering|Material|SetVectorParameterValue (Variables|Settings|GetMI_DynamicSkySphere) "CloudSettings" (Utilities|Struct|MakeLinearColor 1.0 _panningspeed _brightness _skytintstregth) :!class /Script/Engine.MaterialInstanceDynamic))

(fn HandleRain
  (bind _returnvalue (Utilities|IsRaining))
  (bind _ns_rain (Variables|Default|GetNS_Rain))
  (bind _drizzleniagarasettings (Variables|Weather|GetDrizzleNiagaraSettings))
  (bind _thunderstormniagarasettings (Variables|Weather|GetThunderstormNiagaraSettings))
  (bind _ns_rain_2 (Variables|Default|GetNS_Rain))
  (bind _ns_rain_3 (Variables|Default|GetNS_Rain))
  (bind _rainniagarasettings (Variables|Weather|GetRainNiagaraSettings))
  (bind _ns_rain_4 (Variables|Default|GetNS_Rain))
  (bind (_rainvelocity _rainspawnrate) (Utilities|Struct|BreakS_RainNiagaraSettings _rainniagarasettings))
  (bind (_rainvelocity_2 _rainspawnrate_2) (Utilities|Struct|BreakS_DrizzleNiagaraSettings _drizzleniagarasettings))
  (bind (_rainvelocity_3 _rainspawnrate_3) (Utilities|Struct|BreakS_ThunderstormNiagaraSettings _thunderstormniagarasettings))
  (Components|Activation|SetAutoActivate _ns_rain _returnvalue)
  (Components|Activation|SetActive _ns_rain _returnvalue _returnvalue)
  (if _returnvalue
    (switch Utilities|FlowControl|Switch|SwitchonEWeatherConditions (Variables|Default|GetWeatherCondition)
      (:Rain
        (Niagara|SetNiagaraVariable(Float) _ns_rain_3 "RainSpawnRate" _rainspawnrate)
        (Class|NiagaraComponent|SetNiagaraVariableVec3 _ns_rain_3 "RainVelocity" _rainvelocity))
      (:Thunderstorm
        (Niagara|SetNiagaraVariable(Float) _ns_rain_4 "RainSpawnRate" _rainspawnrate_3)
        (Class|NiagaraComponent|SetNiagaraVariableVec3 _ns_rain_4 "RainVelocity" _rainvelocity_3))
      (:Drizzle
        (Niagara|SetNiagaraVariable(Float) _ns_rain_2 "RainSpawnRate" _rainspawnrate_2)
        (Class|NiagaraComponent|SetNiagaraVariableVec3 _ns_rain_2 "RainVelocity" _rainvelocity_2)))))